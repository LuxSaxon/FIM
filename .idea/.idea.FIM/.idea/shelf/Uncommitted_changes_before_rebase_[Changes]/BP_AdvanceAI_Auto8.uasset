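; BP_AdvanceAI is an enemy character that fights the player and can be devoured to grant a skill.
; BeginPlay binds its health UI, initializes its GAS melee ability and runs a behavior tree targeting the player; ReadyFight and StopFight toggle combat rotation and a blackboard flag.
; Hit reactions launch it upward with timeline-driven gravity, or sphere-trace to knock back an AI.
; Being devoured kills it and gives the player GE_DevourPoint and its skill.
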(event `self.ReceiveBeginPlay`
  ;[1 1 1] Setup AI behavior
  (`parent.ReceiveBeginPlay`)
  (`self.AI_Setup`))

(event `/Game/ProjectFIM/Blueprints/BP_interface/BPI_ReadToFight.ReadyFight`
  ;[1 1 1] Setup Combat Mode
  (if (not (`self.bIsDead`))
    (`KismetSystemLibrary.Delay` 1.0)
    (`self.CombatStart` self true false true)
    (`KismetSystemLibrary.Delay` 1.0)
    (`BlackboardComponent.SetValueAsBool` (`AIBlueprintHelperLibrary.GetBlackboard` self) "ReadToFight" true)
    (set `self.EXE_BehaviorTree` true)))

(event `/Game/ProjectFIM/Blueprints/BP_interface/BPI_ReadToFight.StopFight`
  ;[1 1 1] Setup Combat Mode
  (`KismetSystemLibrary.Delay` 1.0)
  (`self.CombatStart` self false true false)
  (`BlackboardComponent.SetValueAsBool` (`AIBlueprintHelperLibrary.GetBlackboard` self) "ReadToFight" false)
  (set `self.EXE_BehaviorTree` false))

(event `self.DevourEvent`
  ;[1 1 1] Be Devoured
  (`parent.DevourEvent`)
  (bind _asbp_test_character (cast `/Game/ProjectFIM/Blueprints/BP_BaseClasses/BP_TestCharacter` (`self.Target_Player`)))
  (`self.OnDevour` _asbp_test_character true null))

(event `/Game/ProjectFIM/Blueprints/BP_interface/BPI_BeDevoured.BeDevoured`
  (params (BeDevoured :type Boolean))
  ;[1 1 1] Be Devoured
  (set `self.IsDevour` BeDevoured)
  (if (not (`self.bIsDead`))
    (`self.BP_Die`)
    (bind _asbp_test_character (cast `/Game/ProjectFIM/Blueprints/BP_BaseClasses/BP_TestCharacter` (`GameplayStatics.GetPlayerCharacter` 0)))
    (bind _returnvalue (`AbilitySystemBlueprintLibrary.GetAbilitySystemComponent` _asbp_test_character))
    (`AbilitySystemComponent.BP_ApplyGameplayEffectToTarget` :`self` _returnvalue :`GameplayEffectClass` "/Game/ProjectFIM/Blueprints/Abilities/GE_DevourPoint.GE_DevourPoint_C" :`Target` _returnvalue)
    (`self.GetDevourSkill` _asbp_test_character (`self.TakeSkillCD`) (`self.TakeSkillID`))))

(event `/Game/ProjectFIM/Blueprints/BP_interface/BPI_Possessing.IsPossessing`
  ;[1 1 1] Be Devoured
  (`self.OnPossessing` self)
  (`KismetSystemLibrary.Delay` 3.0))

(event `/Game/ProjectFIM/Blueprints/BP_interface/BPI_AirAttack.OnAirAttack`
  (params (SceneAirAttack :type "SceneComponent Object Reference") (IsAirAttack :type Boolean))
  ;[1 1 1] Be Devoured
  (`self.KnockUp` SceneAirAttack (0.0 0.0 950.0) (`NavMovementComponent.IsFalling` (`self.CMComp`)))
  (bind (_direction _baketo50) (`Timeline|Timeline` :!via `PlayFromStart`)
    (:`Update`
      (set `CharacterMovementComponent.GravityScale` _baketo50 (`self.CharacterMovement`)))))

(event `/Game/ProjectFIM/Blueprints/BP_interface/BPI_KnockBack.OnKnockBack`
  (params (WorldLocation :type "Vector Structure") (WorldRotation :type "Vector Structure"))
  ;[1 1 1] Be Devoured
  (`self.KnockBack` WorldLocation WorldLocation WorldRotation WorldRotation))

(event `/Game/ProjectFIM/Blueprints/BP_interface/BPI_AirNormalAttack.OnAirNormalAttack`
  ;[1 1 1] Be Devoured
  (`self.KnockUp_NormalAttack` null (0.0 0.0 400.0) (`NavMovementComponent.IsFalling` (`self.CMComp`)))
  (bind (_direction _baketo50) (`Timeline|Timeline_0` :!via `PlayFromStart`)
    (:`Update`
      (set `CharacterMovementComponent.GravityScale` _baketo50 (`self.CharacterMovement`)))))

(fn `AI_Setup`
  (bind _asumg_enemy_ui (cast `/Game/ProjectFIM/Blueprints/UI/UMG_EnemyUI` (`WidgetComponent.GetWidget` (`self.HealthBar`))))
  (set `/Game/ProjectFIM/Blueprints/UI/UMG_EnemyUI.UMG_Owner` self _asumg_enemy_ui)
  (`self.InitializeAttributes` "/Game/ProjectFIM/Blueprints/Abilities/GA_AI_Melee.GA_AI_Melee_C")
  (`AIController.RunBehaviorTree` (`AIBlueprintHelperLibrary.GetAIController` self) "/Game/ProjectFIM/Blueprints/AdvanceAI/BT_AdvanceAI.BT_AdvanceAI")
  (bind _returnvalue (`GameplayStatics.GetActorOfClass` "/Game/ProjectFIM/Blueprints/BP_BaseClasses/BP_TestCharacter.BP_TestCharacter_C"))
  (bind _output_get (set `self.Target_Player` _returnvalue))
  (`BlackboardComponent.SetValueAsObject` (`AIBlueprintHelperLibrary.GetBlackboard` self) "Target" _output_get))

(fn `KnockBack`
  (params (WorldLocation :type "Vector Structure") (WorldLocation_2 :type "Vector Structure") (WorldRotation :type "Vector Structure") (WorldRotation_2 :type "Vector Structure"))
  (bind (_returnvalue_x _returnvalue_y _returnvalue_z) (`KismetMathLibrary.BreakVector` (* WorldRotation 1000.0)))
  (bind (_outhit _returnvalue) (`KismetSystemLibrary.SphereTraceSingleForObjects` :`Start` WorldLocation_2 :`End` (+ WorldLocation (* WorldRotation_2 1000.0)) :`ObjectTypes` (`|MakeArray` "ObjectTypeQuery3" :!type "EObjectTypeQuery Enum") :`DrawDebugType` "ForDuration"))
  (if _returnvalue
    (bind _asbp_advance_ai (cast `/.idea/.idea.FIM/.idea/shelf/Uncommitted_changes_before_rebase_[Changes]/BP_AdvanceAI_Auto8` (`.HitActor` (`GameplayStatics.BreakHitResult` _outhit))))
    (`self.LaunchCharacter` _asbp_advance_ai (`KismetMathLibrary.MakeVector` _returnvalue_x _returnvalue_y (+ _returnvalue_z 700.0)) false false)))

(fn `KnockUp`
  (params (self2 :type "SceneComponent Object Reference") (LaunchVelocity :type "Vector Structure") (InAir :type Boolean))
  (if (not InAir)
    (`self.LaunchCharacter` LaunchVelocity)))

(fn `KnockUp_NormalAttack`
  (params (self2 :type "SceneComponent Object Reference") (LaunchVelocity :type "Vector Structure") (InAir :type Boolean))
  (if InAir
    (`self.LaunchCharacter` LaunchVelocity)))

(fn `UserConstructionScript`)
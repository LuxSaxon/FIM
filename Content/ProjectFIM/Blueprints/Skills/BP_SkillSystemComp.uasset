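; BP_SkillSystemComp is a skill system component that records unlocked skills in a SkillUnlocks map of row name to tier level.
; AddSkill inserts a new skill at tier 1 and always returns true, but re-adds an existing skill with +0, so its tier never rises.
; QuerySkill reports whether a skill is unlocked and its tier, returning false and zero when absent.
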(fn `AddSkill`
  (params (RowName :type String))
  (returns (Success :type Boolean))
  (bind (_value _returnvalue) (`BlueprintMapLibrary.Map_Find` (`self.SkillUnlocks`) RowName))
  (if _returnvalue
    (`BlueprintMapLibrary.Map_Add` (`self.SkillUnlocks`) (`local.RowName`) (+ _value 0))
    (return true)
    (else
      (`BlueprintMapLibrary.Map_Add` (`self.SkillUnlocks`) (`local.RowName`) 1)
      (return true))))

(fn `QuerySkill`
  (params (RowName :type String))
  (returns (Success :type Boolean) (TierLevel :type Integer))
  (bind (_value _returnvalue) (`BlueprintMapLibrary.Map_Find` (`self.SkillUnlocks`) RowName))
  (if _returnvalue
    (return true _value)
    (else
      (return false 0))))
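; Base advanced AI enemy character that fights the player through a behavior tree and a melee gameplay ability.
; On BeginPlay it binds the health bar widget to itself, initializes the melee ability, runs BT_AdvanceAI and stores the test character as the blackboard Target.
; Delayed ReadyFight and StopFight events toggle combat mode, rotation style and the ReadToFight blackboard flag that signals combat readiness to the tree.
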(event `self.ReceiveTick`
  (params (DeltaSeconds :type "Float (single-precision)")))

(event `self.ReceiveBeginPlay`
  ;[1 1 1] Setup AI behavior
  (`parent.ReceiveBeginPlay`)
  (`self.AI_Setup`))

(event `/Game/ProjectFIM/Blueprints/BP_interface/BPI_ReadToFight.ReadyFight`
  ;[1 1 1] Setup Combat Mode
  (`KismetSystemLibrary.Delay` 1.0)
  (`self.CombatStart` self true false true)
  (`KismetSystemLibrary.Delay` 1.0)
  (`BlackboardComponent.SetValueAsBool` (`AIBlueprintHelperLibrary.GetBlackboard` self) "ReadToFight" true)
  (set `self.EXE_BehaviorTree` true))

(event `/Game/ProjectFIM/Blueprints/BP_interface/BPI_ReadToFight.StopFight`
  ;[1 1 1] Setup Combat Mode
  (`KismetSystemLibrary.Delay` 1.0)
  (`self.CombatStart` self false true false)
  (`BlackboardComponent.SetValueAsBool` (`AIBlueprintHelperLibrary.GetBlackboard` self) "ReadToFight" false)
  (set `self.EXE_BehaviorTree` false))

(fn `AI_Setup`
  (bind _asumg_enemy_ui (cast `/Game/ProjectFIM/Blueprints/UI/UMG_EnemyUI` (`WidgetComponent.GetWidget` (`self.HealthBar`))))
  (set `/Game/ProjectFIM/Blueprints/UI/UMG_EnemyUI.UMG_Owner` self _asumg_enemy_ui)
  (`self.InitializeAttributes` "/Game/ProjectFIM/Blueprints/Abilities/GA_AI_Melee.GA_AI_Melee_C")
  (`AIController.RunBehaviorTree` (`AIBlueprintHelperLibrary.GetAIController` self) "/Game/ProjectFIM/Blueprints/AdvanceAI/BT_AdvanceAI.BT_AdvanceAI")
  (bind _returnvalue (`GameplayStatics.GetActorOfClass` "/Game/ProjectFIM/Blueprints/BP_BaseClasses/BP_TestCharacter.BP_TestCharacter_C"))
  (bind _output_get (set `self.Target_Player` _returnvalue))
  (`BlackboardComponent.SetValueAsObject` (`AIBlueprintHelperLibrary.GetBlackboard` self) "Target" _output_get))

(fn `UserConstructionScript`)
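; BP_GhostTrails is a ghost afterimage actor that snapshots the player character's pose and both weapon transforms on BeginPlay.
; It copies the pose from BP_TestCharacter onto its own mesh, places the weapon meshes and disables capsule collision.
; Nested material loops create dynamic MI_GhostTrails instances, assign them to all three meshes and store them.
; An Opacity timeline would fade those materials and destroy the actor, but the graph never starts it.
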(event `self.ReceiveBeginPlay`
  (bind _asbp_test_character (cast `/Game/ProjectFIM/Blueprints/BP_BaseClasses/BP_TestCharacter` (`GameplayStatics.GetPlayerPawn` 0)))
  (set `self.Test Character Ref` _asbp_test_character)
  (`self.Ghost Trails`))

(event `Ghost Trails`
  (bind _test_character_ref (`self.Test Character Ref`))
  (bind _weaponcomp_l (`FIMCharacter.WeaponComp_L` _test_character_ref))
  (bind _weaponcomp_r (`FIMCharacter.WeaponComp_R` _test_character_ref))
  (for _ (`MeshComponent.GetMaterials` (`self.Fantasminha`))
    (for _ (`MeshComponent.GetMaterials` (`self.L_Weapon`))
      (for _ (`MeshComponent.GetMaterials` (`self.R_Weapon`))
        (bind _returnvalue (`KismetMaterialLibrary.CreateDynamicMaterialInstance` "/Game/ProjectFIM/Blueprints/BP_BaseClasses/GhostTail/MI_GhostTrails.MI_GhostTrails"))
        (bind _returnvalue_2 (`KismetArrayLibrary.Array_Add` (`self.DynamicMats`) _returnvalue))
        (`PrimitiveComponent.SetMaterial` (`self.Fantasminha`) _returnvalue_2 _returnvalue)
        (`PrimitiveComponent.SetMaterial` (`self.R_Weapon`) _returnvalue_2 _returnvalue)
        (`PrimitiveComponent.SetMaterial` (`self.L_Weapon`) _returnvalue_2 _returnvalue)
        (`PoseableMeshComponent.CopyPoseFromSkeletalComponent` (`self.Fantasminha`) (`Character.Mesh` (`self.Test Character Ref`)))
        (`SceneComponent.K2_SetWorldLocationAndRotation` (`self.L_Weapon`) (`SceneComponent.K2_GetComponentLocation` _weaponcomp_l) (`SceneComponent.K2_GetComponentRotation` _weaponcomp_l) false false)
        (`SceneComponent.K2_SetWorldLocationAndRotation` (`self.R_Weapon`) (`SceneComponent.K2_GetComponentLocation` _weaponcomp_r) (`SceneComponent.K2_GetComponentRotation` _weaponcomp_r) false false)
        (`PrimitiveComponent.SetCollisionEnabled` (`self.Capsule`) "NoCollision")))))

(fn `OnRep_StoragePose`)

(fn `UserConstructionScript`)
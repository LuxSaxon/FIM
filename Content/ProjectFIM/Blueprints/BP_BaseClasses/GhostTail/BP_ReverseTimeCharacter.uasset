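; BP_ReverseTimeCharacter is a ghost character actor that copies from the player's BP_TestCharacter and fades through an opacity timeline.
; Its GhostCharacter event stores the player pawn as CharacterComp, calls the parent implementation, then starts the Opacity timeline.
; The timeline drives the Opacity scalar parameter on every material in ArrayBodyMaterial and destroys the actor when it finishes.
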(event `self.GhostCharacter`
  (bind _asbp_test_character (cast `/Game/ProjectFIM/Blueprints/BP_BaseClasses/BP_TestCharacter` (`GameplayStatics.GetPlayerPawn` 0)))
  (set `self.CharacterComp` _asbp_test_character)
  (`parent.GhostCharacter`)
  (`TimelineComponent.PlayFromStart` (`self.Opacity`)))

(fn `UserConstructionScript`)
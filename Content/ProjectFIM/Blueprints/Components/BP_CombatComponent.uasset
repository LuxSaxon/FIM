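; Combat component that handles dual sword setup and combat-state messaging for BP_TestCharacter.
; SetUpWeapon finds the character with GetActorOfClass, then spawns left and right swords at its transform, owned by it, and calls OnEquipped on each.
; SetCombatEnable sends a ready-fight or stop-fight message based on its input, without storing the state.
; Simple getters expose left and right weapon references and the combat-start flag.
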(fn `GetWeapon_L`
  (returns (ReturnValue :type "/Game/ProjectFIM/Blueprints/Equipment/BP_BaseWeapon Object Reference"))
  (return (`self.Weapon_L`)))

(fn `GetWeapon_R`
  (returns (ReturnValue :type "/Game/ProjectFIM/Blueprints/Equipment/BP_BaseWeapon Object Reference"))
  (return (`self.Weapon_R`)))

(fn `IsCombatStart?`
  (returns (`bIsCombatStart?` :type Boolean))
  (return (`self.bIsCombatStart?`)))

(fn `SetCombatEnable`
  (params (`bIsCombatStart?` :type Boolean))
  (bind _target (`self.Target`))
  (if `bIsCombatStart?`
    (message `/Game/ProjectFIM/Blueprints/BP_interface/BPI_ReadToFight.ReadyFight` _target)
    (else
      (message `/Game/ProjectFIM/Blueprints/BP_interface/BPI_ReadToFight.StopFight` _target))))

(fn `SetUpWeapon`
  (bind _returnvalue (`GameplayStatics.GetActorOfClass` "/Game/ProjectFIM/Blueprints/BP_BaseClasses/BP_TestCharacter.BP_TestCharacter_C"))
  (bind _output_get (set `self.Player` _returnvalue))
  (`|ExecutionSequence`
    (:`then_0`
      (bind _returnvalue_2 (`|SpawnActorFromClass` "/Game/ProjectFIM/Blueprints/Equipment/BP_BaseSword_L.BP_BaseSword_L_C" (`Actor.GetTransform` _output_get) "Undefined" "OverrideRootScale" _output_get _returnvalue))
      (bind _output_get_2 (set `self.B_Weapon_L` _returnvalue_2))
      (`/Game/ProjectFIM/Blueprints/Equipment/BP_BaseEquippable.OnEquipped` _output_get_2))
    (:`then_1`
      (bind _returnvalue_3 (`|SpawnActorFromClass` "/Game/ProjectFIM/Blueprints/Equipment/BP_BaseSword_R.BP_BaseSword_R_C" (`Actor.GetTransform` _output_get) "Undefined" "OverrideRootScale" _output_get _returnvalue))
      (bind _output_get_3 (set `self.B_Weapon_R` _returnvalue_3))
      (`/Game/ProjectFIM/Blueprints/Equipment/BP_BaseEquippable.OnEquipped` _output_get_3))))
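; Combat component that gives its owning actor a pair of left and right sword weapons.
; SetMainWeapon spawns BP_BaseSword_L and BP_BaseSword_R at the owner's transform, with the owner as Owner and its Instigator passed on.
; Each sword is stored as BWeaponL or BWeaponR and told it is equipped via OnEquipped.
; GetMainWeapon returns both stored weapon references.
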(fn `GetMainWeapon`
  (returns (ReturnValue_L :type "/Game/ProjectFIM/Blueprints/Equipment/BP_BaseWeapon Object Reference") (ReturnValue_R :type "/Game/ProjectFIM/Blueprints/Equipment/BP_BaseWeapon Object Reference"))
  (return (`self.B_Weapon_L`) (`self.B_Weapon_R`)))

(fn `SetMainWeapon`
  (bind _returnvalue (`self.GetOwner`))
  (bind _instigator (`Actor.Instigator` _returnvalue))
  (`|ExecutionSequence`
    (:`then_0`
      (bind _returnvalue_2 (`|SpawnActorFromClass` "/Game/ProjectFIM/Blueprints/Equipment/BP_BaseSword_L.BP_BaseSword_L_C" (`Actor.GetTransform` _returnvalue) "Undefined" "OverrideRootScale" _returnvalue _instigator))
      (bind _output_get (set `self.B_Weapon_L` _returnvalue_2))
      (`/Game/ProjectFIM/Blueprints/Equipment/BP_BaseEquippable.OnEquipped` _output_get))
    (:`then_1`
      (bind _returnvalue_3 (`|SpawnActorFromClass` "/Game/ProjectFIM/Blueprints/Equipment/BP_BaseSword_R.BP_BaseSword_R_C" (`Actor.GetTransform` _returnvalue) "Undefined" "OverrideRootScale" _returnvalue _instigator))
      (bind _output_get_2 (set `self.B_Weapon_R` _returnvalue_3))
      (`/Game/ProjectFIM/Blueprints/Equipment/BP_BaseEquippable.OnEquipped` _output_get_2))))
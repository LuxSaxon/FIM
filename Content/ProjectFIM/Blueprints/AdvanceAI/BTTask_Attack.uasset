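; Behavior tree task that makes a BP_AdvanceAI pawn perform a melee attack through the Gameplay Ability System.
; On execute it ends sprinting, activates GA_AI_Melee unless the pawn is hit, and finishes without waiting for the ability to end.
; On abort it randomizes the pawn's AttackNum unless it is hit, and calls FinishExecute rather than FinishAbort.
; Both events report failure when the pawn is hit or the cast fails.
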(event `self.ReceiveExecuteAI`
  (params (OwnerController :type "AIController Object Reference") (ControlledPawn :type "Pawn Object Reference"))
  ;[1 1 1] Execute Attack
  (bind _asbp_advance_ai (cast `/Game/ProjectFIM/Blueprints/BP_BaseClasses/BP_AdvanceAI_Auto8` ControlledPawn)
    (:`then`
      (`FIMCharacter.SprintEnd` _asbp_advance_ai)
      (if (`FIMCharacter.bIsHitted` _asbp_advance_ai)
        (`self.FinishExecute` false)
        (else
          (`AbilitySystemComponent.TryActivateAbilityByClass` (`FIMCharacter.AbilitySystemComp` _asbp_advance_ai) "/Game/ProjectFIM/Blueprints/Abilities/GA_AI_Melee.GA_AI_Melee_C" true)
          (`self.FinishExecute` true))))
    (:`CastFailed`
      (`self.FinishExecute` false))))

(event `self.ReceiveAbortAI`
  (params (OwnerController :type "AIController Object Reference") (ControlledPawn :type "Pawn Object Reference"))
  ;[1 1 1] Conculate Attack Number
  (bind _asbp_advance_ai (cast `/Game/ProjectFIM/Blueprints/BP_BaseClasses/BP_AdvanceAI_Auto8` ControlledPawn)
    (:`then`
      (if (`FIMCharacter.bIsHitted` _asbp_advance_ai)
        (`self.FinishExecute` false)
        (else
          (set `FIMCharacter.Attack_Num` (`KismetMathLibrary.RandomIntegerInRange` 0 3) _asbp_advance_ai)
          (`self.FinishExecute` true))))
    (:`CastFailed`
      (`self.FinishExecute` false))))
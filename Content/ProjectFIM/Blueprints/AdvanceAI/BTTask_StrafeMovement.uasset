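; Behavior Tree task that makes a BP_AI pawn strafe sideways while facing its target player.
; On execute it randomly picks right or left as the movement direction.
; Each tick it ends sprinting, snaps the pawn's rotation toward TargetPlayer and adds movement input along its right vector.
; A random delay of a few seconds, started from tick, finishes the task successfully.
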(event `self.ReceiveExecuteAI`
  (params (OwnerController :type "AIController Object Reference") (ControlledPawn :type "Pawn Object Reference"))
  ;[1 1 1] Is Right or Left Movement?
  (if (== (`KismetMathLibrary.RandomIntegerInRange` 0 1) 0)
    (set `self.Scale Value` 1.0)
    (else
      (set `self.Scale Value` -1.0))))

(event `self.ReceiveTickAI`
  (params (OwnerController :type "AIController Object Reference") (ControlledPawn :type "Pawn Object Reference") (DeltaSeconds :type "Float (single-precision)"))
  ;[1 1 1] Execute AI Straft Movement and Focus Player
  (bind _asbp_ai (cast `/Game/ProjectFIM/Blueprints/AdvanceAI/BP_AI` ControlledPawn))
  (`FIMCharacter.SprintEnd` _asbp_ai)
  (`Actor.K2_SetActorRotation` _asbp_ai (`KismetMathLibrary.FindLookAtRotation` (`Actor.K2_GetActorLocation` _asbp_ai) (`Actor.K2_GetActorLocation` (`/Game/ProjectFIM/Blueprints/AdvanceAI/BP_AI.Target_Player` _asbp_ai))) false)
  (`Pawn.AddMovementInput` _asbp_ai (`Actor.GetActorRightVector` _asbp_ai) (`self.Scale Value`) false)
  (`KismetSystemLibrary.Delay` (`KismetMathLibrary.Conv_IntToDouble` (`KismetMathLibrary.RandomIntegerInRange` 3 6)))
  (`self.FinishExecute` true))
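; Behavior tree task that makes an AI character randomly either dash or block after ending its sprint.
; Dash picks random -1 to 1 inputs on two axes, scales them by DashDistance, then plays a montage and launches the character along world X/Y.
; Block sets IsBlock, waits a random few seconds, then sets it true again rather than clearing it.
; Both branches finish successfully after their delay.
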(event `self.ReceiveExecuteAI`
  (params (OwnerController :type "AIController Object Reference") (ControlledPawn :type "Pawn Object Reference"))
  (bind _returnvalue (`KismetMathLibrary.RandomIntegerInRange` -1 1))
  (bind _asbp_ai (cast `/Game/ProjectFIM/Blueprints/AdvanceAI/BP_AI` ControlledPawn))
  (`FIMCharacter.SprintEnd` _asbp_ai)
  (if (== (`KismetMathLibrary.RandomIntegerInRange` 0 1) 0)
    (bind _output_get (set `FIMCharacter.InputX` (`KismetMathLibrary.Conv_IntToDouble` _returnvalue) _asbp_ai))
    (bind _output_get_2 (set `FIMCharacter.InputZ` (`KismetMathLibrary.Conv_IntToDouble` _returnvalue) _asbp_ai))
    (`FIMCharacter.PlayDashingMontage` _asbp_ai)
    (bind _dashdistance (`FIMCharacter.DashDistance` _asbp_ai))
    (`Character.LaunchCharacter` _asbp_ai (`KismetMathLibrary.MakeVector` (* _output_get _dashdistance) (* _output_get_2 _dashdistance)) true true)
    (`KismetSystemLibrary.Delay` 0.5)
    (`self.FinishExecute` true)
    (else
      (set `FIMCharacter.bIsBlock` true _asbp_ai)
      (`KismetSystemLibrary.Delay` (`KismetMathLibrary.RandomFloatInRange` 3.0 5.0))
      (set `FIMCharacter.bIsBlock` true _asbp_ai)
      (`self.FinishExecute` true))))
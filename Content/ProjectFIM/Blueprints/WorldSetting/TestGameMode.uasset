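; Test game mode that sets up a ghost replay of the player character from a saved recording.
; On BeginPlay it loads the GhostSaveGame slot, spawns a ghost at the player's mesh if one exists, and opens a Tick gate.
; Tick calls RecordGhost and ReplayGhost, but their transform capture and playback nodes are disconnected, so only the replay index advances.
; SaveGame writes the recorded array to the slot but is not called here.
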(event `self.ReceiveBeginPlay`
  (`|ExecutionSequence`
    (:`then_0`
      (bind _asbp_test_character (cast `/Game/ProjectFIM/Blueprints/BP_BaseClasses/BP_TestCharacter` (`GameplayStatics.GetPlayerPawn` 0)))
      (set `self.As BP Test Character` _asbp_test_character))
    (:`then_1`
      (bind _true (`self.LoadGame`))
      (`self.SpawnGhost` _true)
      (set `FIMCharacter.IsMoving` false (`self.As BP Test Character`))
      (`self.OpenGate`))))

(event `self.ReceiveTick`
  (params (DeltaSeconds :type "Float (single-precision)"))
  (`/Engine/EditorBlueprintResources/StandardMacros.Gate` true :!label _label
    (:`Exit`
      (`self.RecordGhost`)
      (`self.ReplayGhost`))))

(event `OpenGate`
  (goto _label :!via `Open`))

(fn `LoadGame`
  (returns (True :type Boolean))
  (bind _returnvalue (`GameplayStatics.DoesSaveGameExist` (`self.SaveGameSlotName`)))
  (if _returnvalue
    (bind _returnvalue_2 (`GameplayStatics.LoadGameFromSlot` (`self.SaveGameSlotName`)))
    (bind _asghost_save_game (cast `/Game/ProjectFIM/Blueprints/BP_BaseClasses/Replay/GhostSaveGame` _returnvalue_2)
      (:`then`
        (set `self.GhostInfoReplay` (`/Game/ProjectFIM/Blueprints/BP_BaseClasses/Replay/GhostSaveGame.CharacterInfoArray` _asghost_save_game)))
      (:`CastFailed`
        _)))
  (return _returnvalue))

(fn `RecordGhost`)

(fn `ReplayGhost`
  (set `self.Index` (+ (`self.Index`) 1))
  (`|ExecutionSequence`))

(fn `SaveGame`
  (`/Engine/EditorBlueprintResources/StandardMacros.IsValid` (`self.GhostSaveGameObj`)
    (:`Is Valid`
      _)
    (:`Is Not Valid`
      (bind _returnvalue (`GameplayStatics.CreateSaveGameObject` "/Game/ProjectFIM/Blueprints/BP_BaseClasses/Replay/GhostSaveGame.GhostSaveGame_C"))
      (bind _output_get (set `self.GhostSaveGameObj` _returnvalue))))
  (set `/Game/ProjectFIM/Blueprints/BP_BaseClasses/Replay/GhostSaveGame.CharacterInfoArray` (`self.GhostInfoRecord`) _output_get)
  (bind _returnvalue_2 (`GameplayStatics.SaveGameToSlot` (`self.GhostSaveGameObj`) (`self.SaveGameSlotName`)))
  (if _returnvalue_2
    (`KismetSystemLibrary.PrintString` "Game is Save")
    (else
      (`KismetSystemLibrary.PrintString` "Game isn't Save"))))

(fn `SpawnGhost`
  (params (IsTrue :type Boolean))
  (if IsTrue
    (bind _returnvalue (`|SpawnActorFromClass` "/Game/ProjectFIM/Blueprints/BP_BaseClasses/GhostTail/BP_GhostCharacter.BP_GhostCharacter_C" (`SceneComponent.K2_GetComponentToWorld` (`Character.Mesh` (`self.As BP Test Character`))) "AlwaysSpawn" "OverrideRootScale" null null))
    (set `self.GhostPawn` _returnvalue)))

(fn `UserConstructionScript`)
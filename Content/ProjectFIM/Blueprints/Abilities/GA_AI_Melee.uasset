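; GA_AI_Melee is a gameplay ability that performs a melee attack for BP_AdvanceAI characters, ending at once for any other owner.
; It commits, passes four dual-wield combo montages to the AI's NormalAttack, then plays the AI's AMAttack montage.
; During playback it waits for a Char.Skill.Melee.DealDamage gameplay event and applies GE_MeleeDamage to the event's target.
; The ability ends when the montage completes, blends out, is interrupted or is cancelled.
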(event `self.K2_ActivateAbility`
  (bind _asbp_advance_ai (cast `/Game/ProjectFIM/Blueprints/BP_BaseClasses/BP_AdvanceAI_Auto8` (`self.GetOwningActorFromActorInfo`))
    (:`then`
      (`self.K2_CommitAbility`)
      (`FIMCharacter.NormalAttack` _asbp_advance_ai "/Game/ProjectFIM/Animations/Quinn/Normal_Attack_Combo1/Frank_RPG_Dual_Combo01_1_Retargeted_Montage.Frank_RPG_Dual_Combo01_1_Retargeted_Montage" "/Game/ProjectFIM/Animations/Quinn/Normal_Attack_Combo1/Frank_RPG_Dual_Combo01_2_Retargeted_Montage.Frank_RPG_Dual_Combo01_2_Retargeted_Montage" "/Game/ProjectFIM/Animations/Quinn/Normal_Attack_Combo1/Frank_RPG_Dual_Combo01_3_Retargeted_Montage.Frank_RPG_Dual_Combo01_3_Retargeted_Montage" "/Game/ProjectFIM/Animations/Quinn/Normal_Attack_Combo1/Frank_RPG_Dual_Combo01_4_Retargeted_Montage.Frank_RPG_Dual_Combo01_4_Retargeted_Montage")
      (`AbilityTask_PlayMontageAndWait.CreatePlayMontageAndWaitProxy` "None" (`FIMCharacter.AM_Attack` _asbp_advance_ai)
        (:`then`
          (bind (_asynctaskproxy _payload) (`AbilityTask_WaitGameplayEvent.WaitGameplayEvent` (struct :`TagName` "Char.Skill.Melee.DealDamage") null)
            (:`EventReceived`
              (`self.BP_ApplyGameplayEffectToTarget` (`AbilitySystemBlueprintLibrary.AbilityTargetDataFromActor` (`.Target` (break `GameplayEventData` _payload))) "/Game/ProjectFIM/Blueprints/Abilities/GE_MeleeDamage.GE_MeleeDamage_C"))))
        (:`OnCompleted`
          (`self.K2_EndAbility` :!label _label))
        (:`OnBlendOut`
          (goto _label))
        (:`OnInterrupted`
          (goto _label))
        (:`OnCancelled`
          (goto _label))))
    (:`CastFailed`
      (`self.K2_EndAbility`))))
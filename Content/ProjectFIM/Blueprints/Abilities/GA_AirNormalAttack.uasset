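; Gameplay ability for the test character's mid-air normal melee attack, active only while the character is falling.
; It commits, passes three air combo montages to NormalAttack, plays the character's attack montage and launches the character upward, overriding velocity.
; DealDamage gameplay events apply the melee damage effect to the payload target and send an air-attack message to the character's Target.
; The ability ends when the montage finishes or is interrupted.
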(event `self.K2_ActivateAbility`
  (bind _asbp_test_character (cast `/Game/ProjectFIM/Blueprints/BP_BaseClasses/BP_TestCharacter` (`self.GetOwningActorFromActorInfo`))
    (:`then`
      (if (`NavMovementComponent.IsFalling` (`FIMCharacter.CMComp` _asbp_test_character))
        (`self.K2_CommitAbility`)
        (`FIMCharacter.NormalAttack` _asbp_test_character (`|MakeArray` "/Game/ProjectFIM/Animations/Quinn/AirCombo/AM_AirCombo_1.AM_AirCombo_1" "/Game/ProjectFIM/Animations/Quinn/AirCombo/AM_AirCombo_2.AM_AirCombo_2" "/Game/ProjectFIM/Animations/Quinn/AirCombo/AM_AirCombo_3.AM_AirCombo_3" :!type "AnimMontage Object Reference"))
        (`AbilityTask_PlayMontageAndWait.CreatePlayMontageAndWaitProxy` "None" (`FIMCharacter.AM_Attack` _asbp_test_character)
          (:`then`
            (`Character.LaunchCharacter` _asbp_test_character (0.0 0.0 450.0) true true)
            (bind (_asynctaskproxy _payload) (`AbilityTask_WaitGameplayEvent.WaitGameplayEvent` (struct :`TagName` "Char.Skill.Melee.DealDamage") null)
              (:`EventReceived`
                (`self.BP_ApplyGameplayEffectToTarget` (`AbilitySystemBlueprintLibrary.AbilityTargetDataFromActor` (`.Target` (break `GameplayEventData` _payload))) "/Game/ProjectFIM/Blueprints/Abilities/GE_MeleeDamage.GE_MeleeDamage_C")
                (message `/Game/ProjectFIM/Blueprints/BP_interface/BPI_AirNormalAttack.OnAirNormalAttack` (`/Game/ProjectFIM/Blueprints/BP_BaseClasses/BP_TestCharacter.Target` _asbp_test_character)))))
          (:`OnCompleted`
            (`self.K2_EndAbility` :!label _label))
          (:`OnBlendOut`
            (goto _label))
          (:`OnInterrupted`
            (goto _label))
          (:`OnCancelled`
            (goto _label)))))
    (:`CastFailed`
      (`self.K2_EndAbility`))))
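; GA_JumpAttack is a gameplay ability that performs BP_TestCharacter's jumping melee attack, launching the character upward.
; It commits, plays the AM_JumpAttack montage, then after a short delay sets camera lag speed and the AirAttack flag before the launch.
; A DealDamage gameplay event then applies GE_JumpAttack to the payload target and sends an air-attack message to the character's Target.
; Any montage completion, blend-out, interruption or notify ends the ability.
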(event `self.K2_ActivateAbility`
  (bind _asbp_test_character (cast `/Game/ProjectFIM/Blueprints/BP_BaseClasses/BP_TestCharacter` (`self.GetOwningActorFromActorInfo`))
    (:`then`
      (`self.K2_CommitAbility`)
      (`|PlayMontage` (`Character.Mesh` _asbp_test_character) "/Game/ProjectFIM/Animations/Quinn/Skill/AM_JumpAttack.AM_JumpAttack" 1.2
        (:`then`
          (`KismetSystemLibrary.Delay` 0.25)
          (set `SpringArmComponent.CameraLagSpeed` 5.0 (`FIMCharacter.CameraBoom` _asbp_test_character))
          (set `/Game/ProjectFIM/Blueprints/BP_BaseClasses/BP_TestCharacter.AirAttack` true _asbp_test_character)
          (`Character.LaunchCharacter` _asbp_test_character (0.0 0.0 1000.0) false false)
          (bind (_asynctaskproxy _payload) (`AbilityTask_WaitGameplayEvent.WaitGameplayEvent` (struct :`TagName` "Char.Skill.Melee.DealDamage") null)
            (:`EventReceived`
              (`self.BP_ApplyGameplayEffectToTarget` (`AbilitySystemBlueprintLibrary.AbilityTargetDataFromActor` (`.Target` (break `GameplayEventData` _payload))) "/Game/ProjectFIM/Blueprints/Abilities/Skill/JumpAttack/GE_JumpAttack.GE_JumpAttack_C")
              (message `/Game/ProjectFIM/Blueprints/BP_interface/BPI_AirAttack.OnAirAttack` (`/Game/ProjectFIM/Blueprints/BP_BaseClasses/BP_TestCharacter.Target` _asbp_test_character) (`/Game/ProjectFIM/Blueprints/BP_BaseClasses/BP_TestCharacter.SceneAirAttack` _asbp_test_character) true))))
        (:`OnCompleted`
          (`self.K2_EndAbility` :!label _label))
        (:`OnBlendOut`
          (goto _label))
        (:`OnInterrupted`
          (goto _label))
        (:`OnNotifyBegin`
          (goto _label))
        (:`OnNotifyEnd`
          (goto _label))))
    (:`CastFailed`
      (`self.K2_EndAbility`))))